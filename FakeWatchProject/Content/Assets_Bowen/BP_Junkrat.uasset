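; BP_Junkrat is a first-person player Blueprint that implements a Junkrat-style throw-and-detonate mine ability.
; Left Shift spawns a BP_Mine at the MineSpawn point and launches it with an impulse along the camera's forward vector, capped at two active mines.
; A Mines array tracks them in throw order, so right mouse detonates and removes the oldest first, printing a debug message.
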(event `Key|LeftShift`
  (params (Key :type "Key Structure"))
  (bind _returnvalue_location (`KismetMathLibrary.BreakTransform` (`SceneComponent.K2_GetComponentToWorld` (`self.MineSpawn`))))
  ;[1 1 1] Comment
  (:`Pressed`
    (if (< (`KismetArrayLibrary.Array_Length` (`self.Mines`)) 2)
      (bind _returnvalue (`|SpawnActorFromClass` "/Game/Assets_Bowen/BP_Mine.BP_Mine_C" (`KismetMathLibrary.MakeTransform` _returnvalue_location) "Undefined" "OverrideRootScale" null null))
      ;[1 1 1] Comment
      (`KismetArrayLibrary.Array_Add` (`self.Mines`) _returnvalue)
      (`PrimitiveComponent.AddImpulse` (`/Game/Assets_Bowen/BP_Mine.Mine` _returnvalue) (* (`SceneComponent.GetForwardVector` (`self.FirstPersonCameraComponent`)) 2000) "None" false))))

(event `Key|RightMouseButton`
  (params (Key :type "Key Structure"))
  (bind _mines (`self.Mines`))
  (bind _output (`|GetArrayItem` _mines))
  (:`Pressed`
    (if (>= (`KismetArrayLibrary.Array_LastIndex` (`self.Mines`)) 0)
      (`/Game/Assets_Bowen/BP_Mine.Detonate` _output)
      (`KismetSystemLibrary.PrintString` "Detonate !!" true true (struct :`R` 1.0 :`G` 0.071359 :`A` 1.0))
      (`KismetArrayLibrary.Array_RemoveItem` _mines _output))))

(fn `UserConstructionScript`
  (`parent.UserConstructionScript`))